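; BP_PlayerCharacter is the player character Blueprint, whose graphs here hold only debug and development helpers.
; Every tick it reads movement state, horizontal speed and current stamina from its MovementComponent and prints them through the PrintDebugInfo helper.
; The helper formats label-value pairs and displays each for one frame's delta time, giving a live on-screen readout without logging.
; A dev-only Enter key binding applies damage to the character.
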(event EventBeginPlay)

(event Collision|EventActorBeginOverlap
  (params (OtherActor :type Actor%20Object%20Reference)))

(event EventTick
  (params (DeltaSeconds :type Float%20%28single-precision%29))
  (Utilities|PrintDebugInfo "State" (Utilities|String|EnumtoString (Class|CustomMovementComponent|GetMovementState (Variables|Default|GetMovementComponent))))
  (Utilities|PrintDebugInfo "Horizontal Velocity" (Utilities|String|ToString(Float) (Math|Vector2D|Vector2DLength (Class|CustomMovementComponent|GetHorizontalVelocity (Variables|Default|GetMovementComponent)))))
  (Utilities|PrintDebugInfo "CurrentStamina" (Utilities|String|ToString(Float) (Variables|/Script/project_huitz.CustomMovementComponent|GetCurrentStamina (Variables|Default|GetMovementComponent)))))

(event Input|KeyboardEvents|Enter
  (params (Key :type Key%20Structure :default "None"))
  ;[0.4615 0 0 0.1722] DEV ONLY
  (:Pressed
    (Class|CustomCharacterBase|TakeDamage 1.0)))

(fn ConstructionScript)