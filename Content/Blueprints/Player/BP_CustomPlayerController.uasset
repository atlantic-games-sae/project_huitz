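; Player controller that drives the front-end menu flow from login through lobby entry or local test play.
; A successful login swaps the main menu for a newly created lobby select widget.
; Creating or joining a lobby, or starting local test play, removes the relevant menu and background widgets, then switches to game-only input with the cursor hidden.
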(event Custom|OnLocalPlayStarted_TESTING
  (bind _mainmenuwidget_ref (Variables|Default|GetMainMenuWidget_Ref))
  (bind _menubackgroundwidget_ref (Variables|Default|GetMenuBackgroundWidget_Ref))
  (Utilities|IsValid _mainmenuwidget_ref
    (:Is%20Valid
      (Widget|RemovefromParent _mainmenuwidget_ref))
    (:Is%20Not%20Valid
      _))
  (Utilities|IsValid _menubackgroundwidget_ref
    (:Is%20Valid
      (Widget|RemovefromParent _menubackgroundwidget_ref))
    (:Is%20Not%20Valid
      _))
  (Input|SetInputModeGameOnly self false)
  (Variables|Default|SetbShowMouseCursor false))

(event EventOnSuccessfulLogin
  (bind _mainmenuwidget_ref (Variables|Default|GetMainMenuWidget_Ref))
  (Utilities|IsValid _mainmenuwidget_ref
    (:Is%20Valid
      (Widget|RemovefromParent _mainmenuwidget_ref))
    (:Is%20Not%20Valid
      _))
  (bind _returnvalue (UserInterface|CreateWidget "/Game/UI/WBP_LobbySelect_Testing.WBP_LobbySelect_Testing_C" self))
  (bind _output_get (Variables|Default|SetLobbySelectWidget_Ref _returnvalue))
  (UserInterface|Viewport|AddtoViewport _output_get 1))

(event EventOnLobbyCreated
  (bind _lobbyselectwidget_ref (Variables|Default|GetLobbySelectWidget_Ref))
  (bind _menubackgroundwidget_ref (Variables|Default|GetMenuBackgroundWidget_Ref))
  (Utilities|IsValid _lobbyselectwidget_ref
    (:Is%20Valid
      (Widget|RemovefromParent _lobbyselectwidget_ref))
    (:Is%20Not%20Valid
      _))
  (Utilities|IsValid _menubackgroundwidget_ref
    (:Is%20Valid
      (Widget|RemovefromParent _menubackgroundwidget_ref))
    (:Is%20Not%20Valid
      _))
  (Input|SetInputModeGameOnly self false)
  (Variables|Default|SetbShowMouseCursor false))

(event EventOnLobbyJoined
  (bind _lobbyselectwidget_ref (Variables|Default|GetLobbySelectWidget_Ref))
  (bind _menubackgroundwidget_ref (Variables|Default|GetMenuBackgroundWidget_Ref))
  (Utilities|IsValid _lobbyselectwidget_ref
    (:Is%20Valid
      (Widget|RemovefromParent _lobbyselectwidget_ref))
    (:Is%20Not%20Valid
      _))
  (Utilities|IsValid _menubackgroundwidget_ref
    (:Is%20Valid
      (Widget|RemovefromParent _menubackgroundwidget_ref))
    (:Is%20Not%20Valid
      _))
  (Input|SetInputModeGameOnly self false)
  (Variables|Default|SetbShowMouseCursor false))

(fn ConstructionScript)